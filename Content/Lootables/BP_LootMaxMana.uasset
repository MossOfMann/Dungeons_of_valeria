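; BP_LootMaxMana is a loot pickup that upgrades the player's maximum mana.
; Its construction script runs the parent's, then flags the item as an upgrade through IsUpgrade.
; When the player overlaps its Box, it passes current and max mana to UpdatePlayerStats and writes the result back to MaxMana.
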(event `self.ReceiveBeginPlay`
  (`parent.ReceiveBeginPlay`))

(event `self.Box.OnComponentBeginOverlap`
  (params (OverlappedComponent :type "PrimitiveComponent Object Reference") (OtherActor :type "Actor Object Reference") (OtherComp :type "PrimitiveComponent Object Reference") (OtherBodyIndex :type Integer) (bFromSweep :type Boolean) (SweepResult :type "HitResult Structure (by ref)"))
  (bind _as_bp_player (`self.As BP Player`))
  (if (== OtherActor (`self.As BP Player`))
    (bind _newamount (`self.UpdatePlayerStats` (`/Game/DMG_System/Player/BP_Player.CurrentMana` _as_bp_player) (`/Game/DMG_System/Player/BP_Player.MaxMana` _as_bp_player)))
    (set `/Game/DMG_System/Player/BP_Player.MaxMana` _newamount _as_bp_player)))

(fn `UserConstructionScript`
  (`parent.UserConstructionScript`)
  (set `self.IsUpgrade` true))