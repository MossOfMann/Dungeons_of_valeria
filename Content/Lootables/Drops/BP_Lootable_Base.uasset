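; Base lootable drop actor that either restores or upgrades a player stat when consumed.
; BeginPlay caches the player and binds a 2D enchant sound to the actor's destruction, while Tick keeps the Box snapped to the static mesh's location.
; UpdatePlayerStats, gated by a DoOnce, returns a raised maximum for upgrades or a clamped refill otherwise, destroying the actor unless a refill finds the stat already full.
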(event `self.ReceiveBeginPlay`
  (bind _asbp_player (cast `/Game/DMG_System/Player/BP_Player` (`GameplayStatics.GetPlayerCharacter` 0)))
  (set `self.As BP Player` _asbp_player)
  (add `self.OnDestroyed` (delegate `OnDestroyed_Event`)))

(event `OnDestroyed_Event` :!signature `self.OnDestroyed`
  (params (DestroyedActor :type "Actor Object Reference"))
  (`GameplayStatics.PlaySound2D` "/Game/SFX/Objects/enchant.enchant" 1.0 1.0 0.0 null null))

(event `self.ReceiveTick`
  (params (DeltaSeconds :type "Float (single-precision)"))
  (bind _returnvalue (`SceneComponent.K2_GetComponentLocation` (`self.StaticMesh`)))
  (`/Engine/EditorBlueprintResources/StandardMacros.DoOnce` false :!label _label
    (:`Completed`
      (if (== _returnvalue (`SceneComponent.K2_GetComponentLocation` (`self.Box`)))
        (goto _label :!via `Reset`)
        (else
          (`SceneComponent.K2_SetWorldLocation` (`self.Box`) _returnvalue false false)
          (goto _label :!via `Reset`))))))

(fn `UpdatePlayerStats`
  (params (CurrentAmount :type "Float (double-precision)") (MaxAmount :type "Float (double-precision)"))
  (returns (NewAmount :type "Float (double-precision)"))
  (`/Engine/EditorBlueprintResources/StandardMacros.DoOnce` false
    (:`Completed`
      (if (`self.IsUpgrade`)
        (`self.K2_DestroyActor`)
        (return (+ MaxAmount 30.0))
        (elif (< CurrentAmount MaxAmount)
          (`self.K2_DestroyActor`)
          (return (`KismetMathLibrary.FClamp` (+ CurrentAmount 20.0) 0.0 MaxAmount))
          (else
            (return CurrentAmount)))))))

(fn `UserConstructionScript`)