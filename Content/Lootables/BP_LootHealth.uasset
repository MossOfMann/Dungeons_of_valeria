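; BP_LootHealth is a health loot pickup that updates the player's health when touched.
; When its Box begins overlapping the cached player reference, it passes the player's current and maximum health to UpdatePlayerStats.
; The result is written directly to Health on the player's BPCDamageSystem component.
; BeginPlay and the construction script only call their parent versions.
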(event `self.ReceiveBeginPlay`
  (`parent.ReceiveBeginPlay`))

(event `self.Box.OnComponentBeginOverlap`
  (params (OverlappedComponent :type "PrimitiveComponent Object Reference") (OtherActor :type "Actor Object Reference") (OtherComp :type "PrimitiveComponent Object Reference") (OtherBodyIndex :type Integer) (bFromSweep :type Boolean) (SweepResult :type "HitResult Structure (by ref)"))
  (bind _as_bp_player (`self.As BP Player`))
  (if (== OtherActor (`self.As BP Player`))
    (bind _health (`/Game/DMG_System/Player/BP_Player.GetCurretHealth` _as_bp_player))
    (bind _maxhealth (`/Game/DMG_System/Player/BP_Player.GetMaxHealth` _as_bp_player))
    (bind _newamount (`self.UpdatePlayerStats` _health _maxhealth))
    (set `/Game/DMG_System/BPC_DamageSystem_.Health` _newamount (`/Game/DMG_System/Player/BP_Player.BPC_DamageSystem_` _as_bp_player))))

(fn `UserConstructionScript`
  (`parent.UserConstructionScript`))