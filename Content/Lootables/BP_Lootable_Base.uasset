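; Base lootable actor for pickups that either refill or upgrade a player stat.
; On BeginPlay it caches the player character as BP_Player.
; UpdatePlayerStats takes current and max amounts and, behind a DoOnce, returns either a raised maximum for upgrades or a refilled amount capped at max.
; The actor destroys itself when used, except a refill when the stat is already full, which returns the amount unchanged.
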(event `self.ReceiveBeginPlay`
  (bind _asbp_player (cast `/Game/DMG_System/Player/BP_Player` (`GameplayStatics.GetPlayerCharacter` 0)))
  (set `self.As BP Player` _asbp_player))

(fn `UpdatePlayerStats`
  (params (CurrentAmount :type "Float (double-precision)") (MaxAmount :type "Float (double-precision)"))
  (returns (NewAmount :type "Float (double-precision)"))
  (`/Engine/EditorBlueprintResources/StandardMacros.DoOnce` false
    (:`Completed`
      (if (`self.IsUpgrade`)
        (`self.K2_DestroyActor`)
        (return (+ MaxAmount 10.0))
        (elif (< CurrentAmount MaxAmount)
          (`self.K2_DestroyActor`)
          (return (`KismetMathLibrary.FClamp` (+ CurrentAmount 20.0) 0.0 MaxAmount))
          (else
            (return CurrentAmount)))))))

(fn `UserConstructionScript`)