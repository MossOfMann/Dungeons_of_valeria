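; BP_AOEBase is the base area-of-effect actor for spells in the damage system, detecting pawns inside a box around itself.
; Trigger calls SpawnAOE, which runs a box overlap at the actor's location, optionally ignoring the Instigator and drawing a debug box.
; Each overlapped actor is broadcast through the OnAOEOverlapActor dispatcher and its name printed, so this Blueprint applies no effect itself.
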(event `Trigger`
  (`self.SpawnAOE`))

(event `SpawnAOE`
  (if (`self.DrawDebug`)
    (`KismetSystemLibrary.DrawDebugBox` (`self.K2_GetActorLocation`) (`self.HitBoxDimentions`) (struct :`R` 1.0 :`G` 0.368201 :`B` 0.788636 :`A` 1.0) (struct) 2.0 1.0))
  (bind _outactors (`KismetSystemLibrary.BoxOverlapActors` (`self.K2_GetActorLocation`) (`self.HitBoxDimentions`) (`|MakeArray` "ObjectTypeQuery3" :!type "EObjectTypeQuery Enum") null (select `bool` (`self.IgnoreInstagator`) :`true` (`|MakeArray` (`self.GetInstigator`) :!type "Actor Object Reference"))))
  (for _array_element _outactors
    (`self.OnAOEOverlapActor` _array_element)
    (`KismetSystemLibrary.PrintString` (`KismetSystemLibrary.GetDisplayName` _array_element))))

(fn `UserConstructionScript`)