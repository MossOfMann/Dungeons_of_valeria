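; Damage system component that manages its owner's health, death, blocking and regeneration.
; TakeDamage routes each hit through a CanBeDamaged check into blocked, damage or no-damage outcomes, firing blocked, death or damage-response dispatchers.
; Interrupting hits restart regeneration when allowed, which uses a delayed looping timer to restore health up to the maximum.
; BeginPlay also re-calls StartRegeneration on a short repeating delay loop while CanRegen is true.
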(event `self.ReceiveBeginPlay`
  (if (`self.CanRegen`) :!label _label
    (`self.Start Regeneration`))
  (`KismetSystemLibrary.RetriggerableDelay` 0.2)
  (goto _label))

(event `StopRegeneration`
  (`KismetSystemLibrary.K2_ClearAndInvalidateTimerHandle` (stale `Start Regeneration` _returnvalue)))

(event `Start Regeneration`
  (`KismetSystemLibrary.Delay` 5.0)
  (bind _returnvalue (`KismetSystemLibrary.K2_SetTimerDelegate` (delegate `Regeneration`) 0.8 true)))

(event `Regeneration`
  (bind _output_get (set `self.Health` (`KismetMathLibrary.FClamp` (+ (`self.Health`) 1.0) 0.0 (`self.MaxHealth`))))
  (if (== _output_get (`self.MaxHealth`))
    (`self.StopRegeneration`)))

(fn `TakeDamage`
  (params (DamageInfo :type "/Game/DMG_System/S_DamageInfo Structure"))
  (returns (WasDamaged :type Boolean))
  (bind (_amount _damagetype _damageresponse _shoulddamageinvicible _canbeblocked _canbeparried _shouldforceiterrupt) (break `/Game/DMG_System/S_DamageInfo` DamageInfo))
  (`self.CanBeDamaged` _shoulddamageinvicible _canbeblocked
    (:`BlockedDamage`
      (`self.OnBlocked` _canbeparried)
      (return false))
    (:`DoDamage`
      (if (not (`self.IsDead`))
        (bind _output_get (set `self.Health` (- (`self.Health`) _amount)))
        (if (<= _output_get 0.0)
          (set `self.IsDead` true)
          (`self.StopRegeneration`)
          (`self.OnDeath`)
          (return true)
          (elif (or (`self.IsInteruptable`) _shouldforceiterrupt)
            (if (`self.CanRegen`)
              (`self.StopRegeneration`)
              (`self.Start Regeneration`))
            (`self.OnDamageResponse` _damageresponse)
            (return true)))))
    (:`NoDamage`
      (return false))))